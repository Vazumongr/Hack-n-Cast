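; BP_FloatingLight2 is an environment light Blueprint that sets its PointLight's starting intensity on BeginPlay.
; The sign of IntensityFlip picks the start value: MinIntensity when positive, otherwise MaxIntensity.
; A ping-pong pulse, stepping intensity by IntensityRate and delta time and flipping direction at either limit, is present but disconnected.
; Tick is empty, so the intensity stays static after BeginPlay.
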(event `self.ReceiveBeginPlay`
  (bind _pointlight (`self.PointLight`))
  (if (> (`self.IntensityFlip`) 0)
    (`LightComponent.SetIntensity` _pointlight (`self.MinIntensity`))
    (else
      (`LightComponent.SetIntensity` _pointlight (`self.MaxIntensity`)))))

(event `self.ReceiveTick`
  (params (DeltaSeconds :type "Float (single-precision)")))

(fn `UserConstructionScript`)