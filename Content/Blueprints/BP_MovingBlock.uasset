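; BP_MovingBlock is a replicated block actor that moves back and forth along the world X axis.
; On BeginPlay the server enables actor and movement replication, and the construction script makes the actor Movable.
; Each Tick, only the authority offsets the location by Speed without sweeping, reversing Speed whenever an accumulated timer reaches ten seconds.
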(event `self.ReceiveBeginPlay`
  (`/Engine/EditorBlueprintResources/ActorMacros.Switch Has Authority`
    (:`Authority`
      (`self.SetReplicates` true)
      (`self.SetReplicateMovement` true))))

(event `self.ReceiveTick`
  (params (DeltaSeconds :type "Float (single-precision)"))
  (bind _speed (`self.speed`))
  (`/Engine/EditorBlueprintResources/ActorMacros.Switch Has Authority`
    (:`Authority`
      (bind _output_get (set `self.count` (+ (`self.count`) DeltaSeconds)))
      (if (>= _output_get 10.0)
        (set `self.count` 0.0)
        (set `self.speed` (* _speed -1.0)))
      (`self.K2_SetActorLocation` (+ (`self.K2_GetActorLocation`) (`KismetMathLibrary.MakeVector` (* DeltaSeconds _speed)))))))

(fn `UserConstructionScript`
  (`self.SetMobility` "Movable"))