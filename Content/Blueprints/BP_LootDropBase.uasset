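; BP_LootDropBase is a loot drop actor that flies into whoever picks it up.
; OnProximityPickUp stores the picker and sets a flag that lets Tick animate the pickup.
; Each tick subtracts a fixed, frame-rate-dependent step from scale until near zero, and lerps from the current location toward the picker with growing alpha, accelerating the pull.
; The DestroyActor call is unconnected, so the actor is never destroyed here.
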(event `self.OnProximityPickUp`
  (params (PickerUpper :type "Actor Object Reference"))
  (set `self.ActorPickingMeUp` PickerUpper)
  (set `self.bPickedUp` true))

(event `self.ReceiveTick`
  (params (DeltaSeconds :type "Float (single-precision)"))
  (if (`self.bPickedUp`)
    (`self.Shrink`)
    (`self.LerpTowardsGrabber` DeltaSeconds)))

(fn `LerpTowardsGrabber`
  (params (B :type "Float (double-precision)"))
  (bind _output_get (set `self.Alpha` (+ (`self.Alpha`) (* (`self.LerpRate`) B))))
  (`self.K2_SetActorLocation` (`KismetMathLibrary.VLerp` (`self.K2_GetActorLocation`) (`self.K2_GetActorLocation` (`self.ActorPickingMeUp`)) _output_get)))

(fn `Shrink`
  (bind _returnvalue (`self.GetActorScale3D`))
  (if (not (== _returnvalue (0.0 0.0 0.0) :`ErrorTolerance` 0.001))
    (`self.SetActorScale3D` (- _returnvalue (`self.ShrinkRate`)))))

(fn `UserConstructionScript`)