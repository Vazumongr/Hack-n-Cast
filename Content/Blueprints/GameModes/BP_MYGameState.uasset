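; BP_MYGameState is a game state for a wave-based survival mode that relays wave changes and drop spawning.
; Its wave started and ended events pass the current wave number to player 0's BP_PlayerController to update the wave counter, with leftover "Hello" debug prints.
; SpawnDrops forwards the call to BP_SurvivalGameMode, doing nothing if the game mode cast fails.
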(event `self.WaveStarted_BIE`
  (params (CurrentWave :type Integer))
  (`KismetSystemLibrary.PrintString` "Hello")
  (bind _asbp_player_controller (cast `/Game/Blueprints/Player/BP_PlayerController` (`GameplayStatics.GetPlayerController` 0))
    (:`then`
      (`/Game/Blueprints/Player/BP_PlayerController.UpdateWaveCounter` _asbp_player_controller CurrentWave))
    (:`CastFailed`
      (`KismetSystemLibrary.PrintString` "Hello" :!label _label))))

(event `self.WaveEnded_BIE`
  (params (CurrentWave :type Integer))
  (bind _asbp_player_controller (cast `/Game/Blueprints/Player/BP_PlayerController` (`GameplayStatics.GetPlayerController` 0))
    (:`then`
      (`/Game/Blueprints/Player/BP_PlayerController.UpdateWaveCounter` _asbp_player_controller CurrentWave))
    (:`CastFailed`
      (goto _label))))

(fn `SpawnDrops`
  (bind _asbp_survival_game_mode (cast `/Game/Blueprints/GameModes/BP_SurvivalGameMode` (`GameplayStatics.GetGameMode`)))
  (`MYSurvivalGameMode.SpawnDrops` _asbp_survival_game_mode))

(fn `UserConstructionScript`)