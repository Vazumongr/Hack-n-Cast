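; Playable Khaimera character Blueprint that binds player inputs to Gameplay Ability System abilities.
; Sacrifice input activates GA_Sacrifice by class on the AbilitySystemComponent, while primary and secondary inputs activate abilities through stored handles.
; BeginPlay and the construction script are empty, and leftover overhead healthbar owner setup and debug print nodes are disconnected.
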(event `self.ReceiveBeginPlay`)

(event `InputAction|Sacrifice`
  (params (Key :type "Key Structure"))
  (:`Pressed`
    (`AbilitySystemComponent.TryActivateAbilityByClass` (`self.AbilitySystemComponent`) "/Game/Abilities/GA_Sacrifice.GA_Sacrifice_C" true)))

(event `InputAction|PrimaryAbility`
  (params (Key :type "Key Structure"))
  (:`Pressed`
    (`self.ActivateAbilityByHandle` (`self.PrimaryAbilityHandle`))))

(event `InputAction|SecondaryAbility`
  (params (Key :type "Key Structure"))
  (:`Pressed`
    (`self.ActivateAbilityByHandle` (`self.SecondaryAbilityHandle`))))

(fn `UserConstructionScript`)