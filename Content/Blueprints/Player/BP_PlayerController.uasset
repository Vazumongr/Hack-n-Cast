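; Player controller for a survival game that creates the HUD at begin play and forwards wave counter updates to it.
; Key presses open the in-game menu through the game instance, create the starting kit selection widget, or trigger loot drops.
; Drop spawning branches on authority, calling the survival game mode on the server and the game state otherwise.
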(event `self.ReceiveBeginPlay`
  (`self.CreateHUD`))

(event `Key|M`
  (params (Key :type "Key Structure"))
  (:`Pressed`
    (bind _asbp_game_instance (cast `/Game/Blueprints/GameModes/BP_GameInstance` (`GameplayStatics.GetGameInstance`)))
    (`MYGameInstance.LoadInGameMenu` _asbp_game_instance)))

(event `Key|O`
  (params (Key :type "Key Structure"))
  (:`Pressed`
    (bind _returnvalue (`|CreateWidget` "/Game/UserInterface/Menus/WBP_StartingKitSelectionMenu.WBP_StartingKitSelectionMenu_C"))
    (`MYMenuWidgetBase.Setup` _returnvalue)
    (set `/Game/UserInterface/Menus/WBP_StartingKitSelectionMenu.OwningController` self _returnvalue)))

(event `Key|U`
  (params (Key :type "Key Structure"))
  (:`Pressed`
    (`self.SpawnLoot`)))

(event `SpawnLoot`
  (`self.SpawnDrops`))

(fn `SpawnDrops`
  (bind _returnvalue (`GameplayStatics.GetGameMode`))
  (bind _returnvalue_2 (`GameplayStatics.GetGameState`))
  (if (`KismetSystemLibrary.IsServer`)
    (if (`KismetSystemLibrary.IsValid` _returnvalue)
      (bind _asbp_survival_game_mode (cast `/Game/Blueprints/GameModes/BP_SurvivalGameMode` _returnvalue))
      (`MYSurvivalGameMode.SpawnDrops` _asbp_survival_game_mode))
    (elif (`KismetSystemLibrary.IsValid` _returnvalue_2)
      (bind _asbp_mygame_state (cast `/Game/Blueprints/GameModes/BP_MYGameState` _returnvalue_2))
      (`/Game/Blueprints/GameModes/BP_MYGameState.SpawnDrops` _asbp_mygame_state))))

(fn `UpdateWaveCounter`
  (params (CurrentWave :type Integer))
  (bind _aswbp_hud (cast `/Game/UserInterface/HUD/WBP_HUD` (`self.HUDWidget`)))
  (`/Game/UserInterface/HUD/WBP_HUD.UpdateWaveCounter` _aswbp_hud CurrentWave))

(fn `UserConstructionScript`)