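; Player character Blueprint that routes player input to Gameplay Ability System activation.
; Sacrifice input activates GA_Sacrifice by class, while primary and secondary inputs activate abilities through stored handles that are not assigned in these graphs.
; Debug hooks show the ability system overlay on BeginPlay and cycle its category with the E key.
; The construction script and NewFunction_0 are empty.
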(event `self.ReceiveBeginPlay`
  (`KismetSystemLibrary.ExecuteConsoleCommand` "showdebug abilitysystem" null))

(event `InputAction|Sacrifice`
  (params (Key :type "Key Structure"))
  (:`Pressed`
    (`AbilitySystemComponent.TryActivateAbilityByClass` (`self.AbilitySystemComponent`) "/Game/Abilities/GA_Sacrifice.GA_Sacrifice_C" true)))

(event `InputAction|PrimaryAbility`
  (params (Key :type "Key Structure"))
  (:`Pressed`
    (`self.ActivateAbilityByHandle` (`self.PrimaryAbilityHandle`))))

(event `InputAction|SecondaryAbility`
  (params (Key :type "Key Structure"))
  (:`Pressed`
    (`self.ActivateAbilityByHandle` (`self.SecondaryAbilityHandle`))))

(event `Key|E`
  (params (Key :type "Key Structure"))
  (:`Pressed`
    (`KismetSystemLibrary.ExecuteConsoleCommand` "AbilitySystem.Debug.NextCategory" null)))

(fn `NewFunction_0`)

(fn `UserConstructionScript`)