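; BP_Kamehameha is a laser beam effect actor that extends forward over time and stops at blocking geometry.
; On BeginPlay it tints the Niagara beam and impact components.
; Each Tick it line-traces along the forward vector on the Camera channel, drawing debug lines, to set the beam end and to show and position the impact effect.
; Hits clamp the beam length, which regrows at ExtensionRate up to a fixed maximum.
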(event `self.ReceiveBeginPlay`
  (`FXSystemComponent.SetColorParameter` (`self.NiagaraLaser`) "BeamColor" (struct :`R` 0.439657 :`B` 0.300544 :`A` 1.0))
  (`FXSystemComponent.SetColorParameter` (`self.NiagaraImpact`) "ImpactColor" (struct :`R` 0.439657 :`B` 0.300544 :`A` 1.0)))

(event `self.ReceiveTick`
  (params (DeltaSeconds :type "Float (single-precision)"))
  (bind _returnvalue (`self.K2_GetActorLocation`))
  (bind _niagaraimpact (`self.NiagaraImpact`))
  (bind _returnvalue_2 (+ _returnvalue (* (`self.GetActorForwardVector`) (`self.Distance`))))
  (`|ExecutionSequence`
    (:`then_0`
      (set `self.TraceEnd` _returnvalue_2)
      (bind _outhit (`KismetSystemLibrary.LineTraceSingle` :`Start` _returnvalue :`End` _returnvalue_2 :`TraceChannel` "TraceTypeQuery2" :`DrawDebugType` "ForOneFrame"))
      (set `self.bHit` (`GameplayStatics.BreakHitResult` _outhit))
      (set `self.HitLocation` (`.Location` (`GameplayStatics.BreakHitResult` _outhit)))
      (`FXSystemComponent.SetVectorParameter` (`self.NiagaraLaser`) "BeamEnd" (select `bool` (`self.bHit`) :`false` (`self.TraceEnd`) :`true` (`self.HitLocation`)))
      (`SceneComponent.SetVisibility` _niagaraimpact (`self.bHit`) false)
      (`SceneComponent.K2_SetWorldLocation` _niagaraimpact (`self.HitLocation`) false false)
      (if (`self.bHit`)
        (set `self.Distance` (`KismetMathLibrary.VSize` (- (`self.HitLocation`) (`self.K2_GetActorLocation`))))))
    (:`then_1`
      (if (< (`self.Distance`) 5000.0)
        (set `self.Distance` (+ (`self.Distance`) (* DeltaSeconds (`self.ExtensionRate`))))))))

(fn `UserConstructionScript`)