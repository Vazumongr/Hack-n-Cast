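; Player character Blueprint, named as an old version, with a prototype click-to-kill attack and Gameplay Ability System inputs.
; Left mouse calls HitOnServer, which runs a Visibility line trace with no start or end set and destroys any character of this class it hits.
; Sacrifice input activates GA_Sacrifice by class, while SecondaryAbility input activates a stored ability handle.
; KillOnServer and the ability-system debug console commands are leftovers that never run.
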(event `Key|LeftMouseButton`
  (params (Key :type "Key Structure"))
  (:`Pressed`
    (`self.HitOnServer`)))

(event `HitOnServer`
  (bind _outhit (`KismetSystemLibrary.LineTraceSingle` (0.0 0.0 0.0) (0.0 0.0 0.0) "TraceTypeQuery1"))
  (bind _asbp_player_character_old (cast `/Game/BP_PlayerCharacterOld` (`.HitActor` (`GameplayStatics.BreakHitResult` _outhit))))
  (`self.K2_DestroyActor` _asbp_player_character_old))

(event `self.ReceiveActorBeginOverlap`
  (params (OtherActor :type "Actor Object Reference")))

(event `KillOnServer`
  (params (ActorToKill :type "Actor Object Reference"))
  (`self.K2_DestroyActor` ActorToKill))

(event `self.ReceiveBeginPlay`)

(event `InputAction|Sacrifice`
  (params (Key :type "Key Structure"))
  (:`Pressed`
    (`AbilitySystemComponent.TryActivateAbilityByClass` (`self.AbilitySystemComponent`) "/Game/AbilitySystem/GA_Sacrifice.GA_Sacrifice_C" true)))

(event `InputAction|SecondaryAbility`
  (params (Key :type "Key Structure"))
  (:`Pressed`
    (`self.ActivateAbilityByHandle` (`self.SecondaryAbilityHandle`))))

(event `Key|E`
  (params (Key :type "Key Structure")))

(fn `UserConstructionScript`)