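; Gameplay ability for the player character's primary attack, playing a montage chosen by the attack chain counter.
; As the montage starts, a debug-drawn Camera-channel line trace runs forward from near the avatar.
; It applies the first configured effect to the trace target and GE_Sacrifice to the owner.
; The ability ends on montage completion or interruption; the server-only check is disconnected.
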(event `self.K2_ActivateAbility`
  (bind _returnvalue (`self.GetAvatarActorFromActorInfo`))
  (bind _returnvalue_owneractor (break `GameplayAbilityActorInfo` (`self.GetActorInfo`)))
  (bind _returnvalue_2 (+ (`Actor.K2_GetActorLocation` _returnvalue) (0.0 100.0 0.0)))
  (bind _asbp_player_character (cast `/Game/Blueprints/Player/BP_PlayerCharacter` _returnvalue_owneractor)
    (:`then`
      (`AbilityTask_PlayMontageAndWait.CreatePlayMontageAndWaitProxy` "None" (`|GetArrayItem` (`self.Animations`) (`KismetMathLibrary.Conv_ByteToInt` (`MYPlayerCharacter.AttackChainCounter` _asbp_player_character)))
        (:`then`
          (bind _outhit (`KismetSystemLibrary.LineTraceSingle` :`Start` _returnvalue_2 :`End` (+ _returnvalue_2 (* (`Actor.GetActorForwardVector` _returnvalue) (500.0 500.0 500.0))) :`TraceChannel` "TraceTypeQuery2" :`DrawDebugType` "ForDuration"))
          (`self.K2_ApplyGameplayEffectSpecToTarget` (`self.MakeOutgoingGameplayEffectSpec` (`|GetArrayItem` (`self.Effects`))) (`AbilitySystemBlueprintLibrary.AbilityTargetDataFromHitResult` _outhit))
          (`self.BP_ApplyGameplayEffectToOwner` "/Game/Abilities/GE_Sacrifice.GE_Sacrifice_C"))
        (:`OnCompleted`
          (`self.K2_EndAbility` :!label _label))
        (:`OnInterrupted`
          (goto _label))))
    (:`CastFailed`
      (`KismetSystemLibrary.PrintString` "Cast failed"))))