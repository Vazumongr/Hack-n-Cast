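; Gameplay Ability for the player's primary attack, stepping through a three-stage chain on successive activations.
; The AttackChainCounter on BP_PlayerCharacter indexes both the gameplay effect and the montage for the current stage.
; The effect spec goes to the character's SetupWeapons, then the montage plays and the counter immediately advances, wrapping to zero after the third stage.
; The ability ends when the montage completes or is interrupted.
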(event `self.K2_ActivateAbility`
  (bind _returnvalue_owneractor (break `GameplayAbilityActorInfo` (`self.GetActorInfo`)))
  (`KismetSystemLibrary.PrintString` "Activating ability!")
  (bind _asbp_player_character (cast `/Game/Blueprints/Player/BP_PlayerCharacter` _returnvalue_owneractor)
    (:`then`
      (bind _returnvalue (`KismetMathLibrary.Conv_ByteToInt` (`MYPlayerCharacter.AttackChainCounter` _asbp_player_character)))
      (`MYCharacterBase.SetupWeapons` _asbp_player_character (`self.MakeOutgoingGameplayEffectSpec` (`|GetArrayItem` (`self.Effects`) _returnvalue)))
      (`AbilityTask_PlayMontageAndWait.CreatePlayMontageAndWaitProxy` "None" (`|GetArrayItem` (`self.Animations`) _returnvalue)
        (:`then`
          (bind _result (`/Engine/EditorBlueprintResources/StandardMacros.IncrementInt` _returnvalue)
            (:`  `
              (if (> _result 2)
                (set `MYPlayerCharacter.AttackChainCounter` 0 _asbp_player_character)
                (else
                  (set `MYPlayerCharacter.AttackChainCounter` (`KismetMathLibrary.Conv_IntToByte` _result) _asbp_player_character))))))
        (:`OnCompleted`
          (`self.K2_EndAbility` :!label _label))
        (:`OnInterrupted`
          (goto _label))))
    (:`CastFailed`
      (`KismetSystemLibrary.PrintString` "Cast failed"))))